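; Briefcase actor that opens once the handbag, credit card, receptionist PC and phone are picked up, and collects items dropped into its box.
; Tick polls those four pickup flags and plays a timeline that rolls the lid, replaying the Correct sound on every update.
; Box overlap hides a matching phone, credit card, envelope or paper and plays Correct.
; Papers, matched by display name, are counted until three set AllDocPickedup.
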(event OnComponentBeginOverlap(Box)
  (params (OverlappedComponent :type Primitive%20Component%20Object%20Reference) (OtherActor :type Actor%20Object%20Reference) (OtherComp :type Primitive%20Component%20Object%20Reference) (OtherBodyIndex :type Integer) (bFromSweep :type Boolean) (SweepResult :type Hit%20Result%20Structure%20%28by%20ref%29))
  (bind _returnvalue (Utilities|GetDisplayName OtherActor))
  (bind _doccount (Variables|Default|GetDocCount))
  (bind _output_get (Variables|Default|SetGotPhone (== OtherActor (Variables|Default|GetPhone))))
  (bind _output_get_2 (Variables|Default|SetGotCreditCard (== OtherActor (Variables|Default|GetCreditCard))))
  (bind _output_get_3 (Variables|Default|SetGotEnvelope (== OtherActor (Variables|Default|GetEnvelope))))
  (if (Math|Boolean|ORBoolean _output_get_3 _output_get_2 _output_get (Utilities|Enum|Equal(Enum) _returnvalue (Utilities|GetDisplayName (Variables|Default|GetGenericPaper))))
    (Development|SetHiddeninGame (Variables|/Script/Engine.Actor|GetRootComponent OtherActor) true false)
    (Audio|Components|Audio|Play (Variables|Default|GetCorrect) 0.0)
    (if (Utilities|Enum|Equal(Enum) "Generic_paper_Blueprint" _returnvalue)
      (Math|Integer|IncrementInt _doccount
        (:%20%20
          (if (== _doccount 3)
            (Variables|Default|SetAllDocPickedup true)))))))

(event EventTick
  (params (DeltaSeconds :type Float%20%28single-precision%29))
  (bind _asrecep_pc_blueprint (Utilities|Casting|CastToRecep_PC_Blueprint (Variables|Default|GetPC)))
  (bind _ascredit_card_blueprint (Utilities|Casting|CastToCredit_Card_Blueprint (Variables|Default|GetCreditCard)))
  (bind _asphone_blueprint (Utilities|Casting|CastToPhone_Blueprint (Variables|Default|GetPhone)))
  (bind _ashandbag_blueprint (Utilities|Casting|CastToHandbag_Blueprint (Variables|Default|GetHandbag)))
  (if (Math|Boolean|ANDBoolean (Variables|/Game/Blueprints/Handbag_Blueprint.Handbag_Blueprint_C|GetIsPickUp _ashandbag_blueprint) (Variables|/Game/Blueprints/Credit_Card_Blueprint.Credit_Card_Blueprint_C|GetIsPickedUp _ascredit_card_blueprint) (Variables|/Game/Blueprints/Recep_PC_Blueprint.Recep_PC_Blueprint_C|GetIs%20Picked%20Up _asrecep_pc_blueprint) (Variables|/Game/Blueprints/Phone_Blueprint.Phone_Blueprint_C|GetIsPickedUp _asphone_blueprint))
    (bind _openamount (Timeline|OpenBriefcase Play)
      (:Update
        (Transformation|SetRelativeRotation (Variables|Default|GetBriefcase_Top) (Math|Rotator|MakeRotator _openamount 0.0 0.0) false false)
        (Audio|Components|Audio|Play (Variables|Default|GetCorrect) 0.0)))))

(fn ConstructionScript)