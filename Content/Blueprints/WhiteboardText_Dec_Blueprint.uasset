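; Whiteboard text decal Blueprint that disappears when rubbed out with the Rubber actor.
; A Box overlap sets RubbedOut by comparing the overlapping actor to Rubber and plays Wipe on any overlap.
; When the actor is the Rubber, it plays Wipe again, waits briefly, then hides the decal and its children in game.
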(event OnComponentBeginOverlap(Box)
  (params (OverlappedComponent :type Primitive%20Component%20Object%20Reference) (OtherActor :type Actor%20Object%20Reference) (OtherComp :type Primitive%20Component%20Object%20Reference) (OtherBodyIndex :type Integer) (bFromSweep :type Boolean) (SweepResult :type Hit%20Result%20Structure%20%28by%20ref%29))
  (bind _output_get (Variables|Default|SetRubbedOut (== OtherActor (Variables|Default|GetRubber))))
  (Audio|Components|Audio|Play (Variables|Default|GetWipe) 0.0)
  (if _output_get
    (Audio|Components|Audio|Play (Variables|Default|GetWipe) 0.0)
    (Utilities|FlowControl|Delay 1.0)
    (Development|SetHiddeninGame (Variables|Decal|GetDecal) true true)))

(fn ConstructionScript)