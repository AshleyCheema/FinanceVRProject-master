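; A VR credit card prop that a motion controller can pick up and drop.
; Pickup turns off mesh physics, attaches the root to the given component at its world transform, records the result in IsPickedUp and sets a physical material override.
; A DoOnce then plays the Correct component, apparently a success sound, on the first pickup only.
; Drop re-enables physics and detaches the actor, leaving IsPickedUp unchanged.
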(event EventPickup
  (params (AttachTo :type Scene%20Component%20Object%20Reference))
  (Physics|SetSimulatePhysics (Variables|Debug|GetStaticMeshComponent) false)
  (bind _returnvalue (Transformation|AttachComponentToComponent (VehicleSound|GetRootComponent) AttachTo "None" "KeepWorld" "KeepWorld" "KeepWorld" false))
  (Variables|Default|SetIsPickedUp _returnvalue)
  (Class|PrimitiveComponent|SetPhysMaterialOverride (Variables|Debug|GetStaticMeshComponent) "/Game/Material/123.123")
  (Utilities|FlowControl|DoOnce false
    (:Completed
      (Audio|Components|Audio|Play (Variables|Default|GetCorrect) 0.0))))

(event EventDrop
  (Physics|SetSimulatePhysics (Variables|Debug|GetStaticMeshComponent) true)
  (Transformation|DetachFromActor "KeepWorld" "KeepWorld" "KeepWorld"))

(fn ConstructionScript)