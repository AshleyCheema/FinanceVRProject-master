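; BP_FilingCabinet2 is a filing cabinet that collects paper documents and opens its drawer once two are filed.
; Overlaps on CollisionVolume match actors by the display name "Generic_paper", hide their root component, play Correct and increment DocCount.
; On the second count it sets AllDocs and runs the Open_Drawer timeline, which moves FilingCabinetDrawer and replays Correct on every update.
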(event OnComponentBeginOverlap(CollisionVolume)
  (params (OverlappedComponent :type Primitive%20Component%20Object%20Reference) (OtherActor :type Actor%20Object%20Reference) (OtherComp :type Primitive%20Component%20Object%20Reference) (OtherBodyIndex :type Integer) (bFromSweep :type Boolean) (SweepResult :type Hit%20Result%20Structure%20%28by%20ref%29))
  (bind _doccount (Variables|Default|GetDocCount))
  (if (Utilities|Enum|Equal(Enum) "Generic_paper" (Utilities|GetDisplayName OtherActor))
    (Development|SetHiddeninGame (Variables|/Script/Engine.Actor|GetRootComponent OtherActor) true false)
    (Audio|Components|Audio|Play (Variables|Default|GetCorrect) 0.0)
    (Math|Integer|IncrementInt _doccount
      (:%20%20
        (if (== _doccount 2)
          (Variables|Default|SetAllDocs true)
          (bind _openamount (Timeline|Open_Drawer Play)
            (:Update
              (Transformation|SetRelativeLocation (Variables|Default|GetFilingCabinet_Drawer) _openamount false false)
              (Audio|Components|Audio|Play (Variables|Default|GetCorrect) 0.0))))))))

(fn ConstructionScript)