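; Safe bin Blueprint that acts as a shredder, tracking documents dropped into it.
; Any actor overlapping its Box has its root component hidden, without propagating to children or being destroyed, and triggers the Shredder and UIConfirmation audio.
; Only an actor whose display name exactly matches BinBag_US_Blueprint increments DocCount, which sets the AllDocs flag on reaching three.
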(event OnComponentBeginOverlap(Box)
  (params (OverlappedComponent :type Primitive%20Component%20Object%20Reference) (OtherActor :type Actor%20Object%20Reference) (OtherComp :type Primitive%20Component%20Object%20Reference) (OtherBodyIndex :type Integer) (bFromSweep :type Boolean) (SweepResult :type Hit%20Result%20Structure%20%28by%20ref%29))
  (bind _doccount (Variables|Default|GetDocCount))
  (Development|SetHiddeninGame (Variables|/Script/Engine.Actor|GetRootComponent OtherActor) true false)
  (Audio|Components|Audio|Play (Variables|Default|GetShredder) 0.0)
  (if (Utilities|Enum|Equal(Enum) "BinBag_US_Blueprint" (Utilities|GetDisplayName OtherActor))
    (Math|Integer|IncrementInt _doccount
      (:%20%20
        (if (== _doccount 3)
          (Variables|Default|SetAllDocs true))))))

(fn ConstructionScript)